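; Test actor that exercises communication with BP_ThirdPersonCharacter through an event dispatcher and a box trigger, printing the results.
; On BeginPlay it binds a custom event to the player character's NewEventDispatcher, which prints a debug string when fired.
; When the character overlaps the Box, it prints the dot product of both forward vectors, then calls DeadMessage on the character and prints the returned value.
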(event OnComponentBeginOverlap(Box)
  (params (OverlappedComponent :type Primitive%20Component%20Object%20Reference) (OtherActor :type Actor%20Object%20Reference) (OtherComp :type Primitive%20Component%20Object%20Reference) (OtherBodyIndex :type Integer) (bFromSweep :type Boolean) (SweepResult :type Hit%20Result%20Structure%20%28by%20ref%29))
  (bind _asbp_third_person_character (Utilities|Casting|CastToBP_ThirdPersonCharacter OtherActor))
  (Development|PrintString (Utilities|String|ToString(Float) (Math|Vector|DotProduct (Transformation|GetActorForwardVector _asbp_third_person_character) (Transformation|GetActorForwardVector))))
  (bind _num (Class|BPIDead|Dead(Message) OtherActor (Variables|Default|GetNewVar)))
  (Development|PrintString (Utilities|String|ToString(Float) _num)))

(event Custom|自定义事件
  (Development|PrintString "shoudaoming"))

(event EventBeginPlay
  (bind _asbp_third_person_character (Utilities|Casting|CastToBP_ThirdPersonCharacter (Game|GetPlayerCharacter 0)))
  (EventDispatchers|BindEventtoNewEventDispatcher _asbp_third_person_character (delegate Custom|自定义事件)))

(event Collision|EventActorBeginOverlap
  (params (OtherActor :type Actor%20Object%20Reference)))

(event EventTick
  (params (DeltaSeconds :type Float%20%28single-precision%29)))

(fn ConstructionScript)